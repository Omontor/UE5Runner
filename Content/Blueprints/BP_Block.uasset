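; Endless-runner track segment with four obstacle lanes, two sidewalk and two street, where hitting an obstacle quits the game.
; BeginPlay randomly assigns obstacle meshes, then spawns a coin in a random lane if it is empty.
; Tick moves the street obstacles and line-traces to the neighboring block, clearing lane spawn flags where it has trucks.
; When the player overlaps its trigger, the GameMode adds a block and this one destroys itself after a delay.
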(event `self.ReceiveBeginPlay`
  (`self.SpawnObstacles`)
  (`self.SpawnCoins`))

(event `self.ReceiveTick`
  (params (DeltaSeconds :type "Float (single-precision)"))
  (bind _frontblock (`self.CheckFrontBlock`))
  (`/Engine/EditorBlueprintResources/StandardMacros.IsValid` _frontblock
    (:`Is Valid`
      (set `self.SpawnLane2Car` (not (== (`StaticMeshComponent.StaticMesh` (`/Game/Blueprints/BP_Block.Obstacle 2` _frontblock)) "/Game/Vehiculos/SM_vh_truck.SM_vh_truck")))
      (set `self.SpawnLane3Car` (not (== (`StaticMeshComponent.StaticMesh` (`/Game/Blueprints/BP_Block.Obstacle 3` _frontblock)) "/Game/Vehiculos/SM_vh_truck.SM_vh_truck"))))
    (:`Is Not Valid`
      _))
  (`self.MoveCars`))

(event `self.OverlapBox.OnComponentBeginOverlap`
  (params (OverlappedComponent :type "PrimitiveComponent Object Reference") (OtherActor :type "Actor Object Reference") (OtherComp :type "PrimitiveComponent Object Reference") (OtherBodyIndex :type Integer) (bFromSweep :type Boolean) (SweepResult :type "HitResult Structure (by ref)"))
  (cast `/Game/ThirdPerson/Blueprints/BP_ThirdPersonCharacter` OtherActor)
  (bind _asbp_third_person_game_mode (cast `/Game/ThirdPerson/Blueprints/BP_ThirdPersonGameMode` (`GameplayStatics.GetGameMode`)))
  (`/Game/ThirdPerson/Blueprints/BP_ThirdPersonGameMode.AddBlock` _asbp_third_person_game_mode true)
  (`KismetSystemLibrary.Delay` 5.0)
  (`self.K2_DestroyActor`))

(event `self.Obstacle 1.OnComponentBeginOverlap`
  (params (OverlappedComponent :type "PrimitiveComponent Object Reference") (OtherActor :type "Actor Object Reference") (OtherComp :type "PrimitiveComponent Object Reference") (OtherBodyIndex :type Integer) (bFromSweep :type Boolean) (SweepResult :type "HitResult Structure (by ref)"))
  (cast `/Game/ThirdPerson/Blueprints/BP_ThirdPersonCharacter` OtherActor)
  (`KismetSystemLibrary.QuitGame` null "Quit"))

(event `self.Obstacle 2.OnComponentBeginOverlap`
  (params (OverlappedComponent :type "PrimitiveComponent Object Reference") (OtherActor :type "Actor Object Reference") (OtherComp :type "PrimitiveComponent Object Reference") (OtherBodyIndex :type Integer) (bFromSweep :type Boolean) (SweepResult :type "HitResult Structure (by ref)"))
  (cast `/Game/ThirdPerson/Blueprints/BP_ThirdPersonCharacter` OtherActor)
  (`KismetSystemLibrary.QuitGame` null "Quit"))

(event `self.Obstacle 3.OnComponentBeginOverlap`
  (params (OverlappedComponent :type "PrimitiveComponent Object Reference") (OtherActor :type "Actor Object Reference") (OtherComp :type "PrimitiveComponent Object Reference") (OtherBodyIndex :type Integer) (bFromSweep :type Boolean) (SweepResult :type "HitResult Structure (by ref)"))
  (cast `/Game/ThirdPerson/Blueprints/BP_ThirdPersonCharacter` OtherActor)
  (`KismetSystemLibrary.QuitGame` null "Quit"))

(event `self.Obstacle 4.OnComponentBeginOverlap`
  (params (OverlappedComponent :type "PrimitiveComponent Object Reference") (OtherActor :type "Actor Object Reference") (OtherComp :type "PrimitiveComponent Object Reference") (OtherBodyIndex :type Integer) (bFromSweep :type Boolean) (SweepResult :type "HitResult Structure (by ref)"))
  (cast `/Game/ThirdPerson/Blueprints/BP_ThirdPersonCharacter` OtherActor)
  (`KismetSystemLibrary.QuitGame` null "Quit"))

(fn `CheckFrontBlock`
  (returns (FrontBlock :type "/Game/Blueprints/BP_Block Object Reference"))
  (bind _returnvalue (`self.K2_GetActorLocation`))
  (bind _outhit (`KismetSystemLibrary.LineTraceSingle` _returnvalue (+ _returnvalue (* (`self.GetActorRightVector`) -400.0)) "TraceTypeQuery1"))
  (bind _asbp_block (cast `/Game/Blueprints/BP_Block` (`.HitActor` (`GameplayStatics.BreakHitResult` _outhit))))
  (return _asbp_block))

(fn `MoveCars`
  (bind _obstacle_2 (`self.Obstacle 2`))
  (bind _obstacle_3 (`self.Obstacle 3`))
  (`SceneComponent.K2_SetWorldLocation` _obstacle_2 (+ (`SceneComponent.K2_GetComponentLocation` _obstacle_2) (* (0.0 -1.0 0.0) 10.0)) false false)
  (`SceneComponent.K2_SetWorldLocation` _obstacle_3 (+ (`SceneComponent.K2_GetComponentLocation` _obstacle_3) (* (0.0 -1.0 0.0) 10.0)) false false))

(fn `SpawnCoins`
  (bind _returnvalue (select `int` (`self.coinLane`) :`0` (`self.Obstacle 1`) :`1` (`self.Obstacle 2`) :`2` (`self.Obstacle 3`) :`3` (`self.Obstacle 4`)))
  (set `self.coinLane` (`KismetMathLibrary.RandomIntegerInRange` 0 3))
  (`/Engine/EditorBlueprintResources/StandardMacros.IsValid` (`StaticMeshComponent.StaticMesh` _returnvalue)
    (:`Is Not Valid`
      (`|SpawnActorFromClass` "/Game/Blueprints/BP_Coin.BP_Coin_C" (`KismetMathLibrary.MakeTransform` (`SceneComponent.K2_GetComponentLocation` _returnvalue)) "Undefined" "OverrideRootScale" null null))))

(fn `SpawnObstacles`
  (if (`self._SpawnObstacles`)
    (if (== (`KismetMathLibrary.RandomIntegerInRange` 0 1) 0)
      (`|ExecutionSequence`
        (:`then_0`
          (if (== (`KismetMathLibrary.RandomIntegerInRange` 0 1) 0)
            (`StaticMeshComponent.SetStaticMesh` (`self.Obstacle 1`) (`KismetArrayLibrary.Array_Random` (`self.SidewalkMeshes`)))))
        (:`then_1`
          (if (`self.SpawnLane2Car`)
            (if (== (`KismetMathLibrary.RandomIntegerInRange` 0 1) 0)
              (`StaticMeshComponent.SetStaticMesh` (`self.Obstacle 2`) (`KismetArrayLibrary.Array_Random` (`self.StreetMeshes`))))))
        (:`then_2`
          (if (`self.SpawnLane3Car`)
            (if (== (`KismetMathLibrary.RandomIntegerInRange` 0 1) 0)
              (`StaticMeshComponent.SetStaticMesh` (`self.Obstacle 3`) (`KismetArrayLibrary.Array_Random` (`self.StreetMeshes`))))))
        (:`then_3`
          (if (== (`KismetMathLibrary.RandomIntegerInRange` 0 1) 0)
            (`StaticMeshComponent.SetStaticMesh` (`self.Obstacle 4`) (`KismetArrayLibrary.Array_Random` (`self.SidewalkMeshes`)))))))))

(fn `UserConstructionScript`)